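; BP_Trigger is a trigger actor that advances the train along its spline route when the VR pawn overlaps it.
; On BeginPlay it finds the BP_Train in the level and stores a reference.
; On overlap, if the train has finished travelling, it increments the train's spline index, calls MoveObject and destroys itself.
; At the last spline it prints a red GAME OVER message instead.
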(event EventBeginPlay
  (bind _returnvalue (Actor|GetActorOfClass "/Game/Train-Rail/BP_Train.BP_Train_C"))
  (bind _output_get (Variables|Default|SetTrainREF _returnvalue))
  (Development|PrintString (Utilities|GetDisplayName _output_get)))

(event Collision|EventActorBeginOverlap
  (params (OtherActor :type Actor%20Object%20Reference))
  (bind _trainref (Variables|Default|GetTrainREF))
  (Utilities|Casting|CastToVRPawn OtherActor)
  (if (Variables|/Game/Train-Rail/BP_Train.BP_Train_C|GettravelIsFinished _trainref)
    (if (== (Variables|/Game/Train-Rail/BP_Train.BP_Train_C|GetCurrentIndex _trainref) (- (Utilities|Array|Length (Variables|/Game/Train-Rail/BP_Train.BP_Train_C|GetSpline%20Refs _trainref)) 1))
      (Development|PrintString "GAME OVER" true true "(R=1.000000,G=0.000000,B=0.010851,A=1.000000)")
      (else
        (Variables|/Game/Train-Rail/BP_Train.BP_Train_C|SetCurrentIndex _trainref (+ (Variables|/Game/Train-Rail/BP_Train.BP_Train_C|GetCurrentIndex _trainref) 1))
        (Default|MoveObject _trainref)
        (Actor|DestroyActor)))))

(event EventTick
  (params (DeltaSeconds :type Float%20%28single-precision%29)))

(fn ConstructionScript)