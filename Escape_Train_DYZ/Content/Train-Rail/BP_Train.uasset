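; BP_Train is a train actor that rides the spline of the first BP_Rail found in the level, starting on BeginPlay with a sound at its location.
; A timeline, rate-scaled by TimeToComplete, lerps distance along the spline's length.
; Each update sets the actor's transform from that point, taking only world-space X and Y for location and using local-space spline rotation.
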(event Custom|Move%20Object
  (bind _splineref (Variables|Default|GetSplineRef))
  (bind _spline (Variables|/Game/Train-Rail/BP_Rail.BP_Rail_C|GetSpline _splineref))
  (Components|Timeline|SetPlayRate (Variables|Default|GetMove%20Object%20X) (/ 1.0 (Variables|Default|GetTimeToComplete)))
  (bind _move_track (Timeline|Move%20Object%20X Play)
    (:Update
      (Transformation|SetActorTransform (Math|Transform|MakeTransform (Math|Vector|MakeVector (.x (Spline|GetLocationatDistanceAlongSpline _spline (Math|Float|Lerp 0.0 (Spline|GetSplineLength (Variables|/Game/Train-Rail/BP_Rail.BP_Rail_C|GetSpline (Variables|Default|GetSplineRef))) _move_track) "World")) (.y (Spline|GetLocationatDistanceAlongSpline _spline (Math|Float|Lerp 0.0 (Spline|GetSplineLength (Variables|/Game/Train-Rail/BP_Rail.BP_Rail_C|GetSpline (Variables|Default|GetSplineRef))) _move_track) "World")) 0.0) (Spline|GetRotationatDistanceAlongSpline _spline (Math|Float|Lerp 0.0 (Spline|GetSplineLength (Variables|/Game/Train-Rail/BP_Rail.BP_Rail_C|GetSpline (Variables|Default|GetSplineRef))) _move_track) "Local") "1.000000,1.000000,1.000000")))))

(event EventBeginPlay
  (Utilities|FlowControl|Sequence
    (:then_0
      (bind _returnvalue (Actor|GetActorOfClass "/Game/Train-Rail/BP_Rail.BP_Rail_C"))
      (Variables|Default|SetSplineRef _returnvalue)
      (CallFunction|MoveObject))
    (:then_1
      (Audio|PlaySoundatLocation (Variables|Default|GetSound) (Transformation|GetActorLocation) "0, 0, 0" 1.0 1.0 0.0 0 0 0 0))))

(event Collision|EventActorBeginOverlap
  (params (OtherActor :type Actor%20Object%20Reference)))

(event EventTick
  (params (DeltaSeconds :type Float%20%28single-precision%29)))

(fn ConstructionScript)